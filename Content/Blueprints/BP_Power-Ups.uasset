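; BP_Power-Ups is a world pickup for the Insta-Kill, Double Points and Nuke power-ups.
; When a FirstPersonCharacter overlaps it, it passes its PowerUpType to the GunKatta game mode's ActivatePowerUp, then destroys itself.
; The construction script sets the text render label to the selected type's name, while the effects themselves are left to the game mode.
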(event `self.ReceiveActorBeginOverlap`
  (params (OtherActor :type "Actor Object Reference"))
  (cast `/Game/FirstPersonBP/Blueprints/FirstPersonCharacter` OtherActor)
  (bind _asgun_katta (cast `/Game/Blueprints/GunKatta` (`GameplayStatics.GetGameMode`)))
  (`/Game/Blueprints/GunKatta.Activate Power-Up` _asgun_katta (`self.PowerUp-Type`))
  (`self.K2_DestroyActor`))

(fn `UserConstructionScript`
  (locals (`New Text` :type Text))
  (switch `/Game/Enums/E_PowerUps` (`self.PowerUp-Type`)
    (:`NewEnumerator0`
      (set `local.New Text` "Insta-Kill"))
    (:`NewEnumerator1`
      (set `local.New Text` "Double Points"))
    (:`NewEnumerator2`
      (set `local.New Text` "Nuke")))
  (`TextRenderComponent.K2_SetText` (`self.TextRender`) (`local.New Text`)))