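; GunKatta runs the wave-based cat spawning and the timed power-ups of a first-person game.
; A looping timer spawns enemies at every "Spawnable"-tagged SpawnerBoxv2 while cats remain, then advances the wave and recalculates the count once no Kitty actors are left.
; ActivatePower-Up sets Insta-Kill or Double Points flags, adds HUD icons for players and clears the flag after a delay.
; The older random-box spawner and an empty PowerUpActivated event remain.
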(event `self.ReceiveBeginPlay`
  (`self.Spawn Wave`)
  (`KismetSystemLibrary.K2_SetTimerDelegate` (delegate `Spawn Wave`) 10.0 true))

(event `Activate Spawner`
  (bind _spawner_boxes (`self.Spawner Boxes`))
  ;[1 1 1] Old Spawn Method
  (if (> (`self.Cats Left`) 0)
    (`/Game/Cats/SpawnerBoxv2.SpawnCat` (`|GetArrayItem` _spawner_boxes (`KismetMathLibrary.RandomIntegerInRange` 0 (- (`KismetArrayLibrary.Array_Length` _spawner_boxes) 1))) "/Game/Cats/CatTypes/Kitty.Kitty_C")
    (`/Engine/EditorBlueprintResources/StandardMacros.DecrementInt` (`self.Cats Left`))
    (else
      (bind _outactors (`GameplayStatics.GetAllActorsOfClass` "/Game/Cats/CatTypes/Kitty.Kitty_C"))
      (if (== (`KismetArrayLibrary.Array_Length` _outactors) 0)
        (`/Engine/EditorBlueprintResources/StandardMacros.IncrementInt` (`self.Wave #`)
          (:`  `
            (`self.Calculate Cat Number`)))))))

(event `Spawn Wave`
  ;[1 1 1] Spawn Waves
  (if (> (`self.Cats Left`) 0)
    (bind _outactors (`GameplayStatics.GetAllActorsOfClassWithTag` "/Game/Cats/SpawnerBoxv2.SpawnerBoxv2_C" "Spawnable"))
    (for _array_element _outactors
      (bind _asspawner_boxv_2 (cast `/Game/Cats/SpawnerBoxv2` _array_element))
      (`/Game/Cats/SpawnerBoxv2.SpawnCat` _asspawner_boxv_2 (`/Game/Cats/SpawnerBoxv2.EnemyType` _asspawner_boxv_2))
      (`/Engine/EditorBlueprintResources/StandardMacros.DecrementInt` (`self.Cats Left`)))
    (else
      (bind _outactors_2 (`GameplayStatics.GetAllActorsOfClass` "/Game/Cats/CatTypes/Kitty.Kitty_C"))
      (if (== (`KismetArrayLibrary.Array_Length` _outactors_2) 0)
        (`/Engine/EditorBlueprintResources/StandardMacros.IncrementInt` (`self.Wave #`)
          (:`  `
            (`self.Calculate Cat Number`)))))))

(event `Activate Power-Up`
  (params (`Power-Up` :type "/Game/Enums/E_PowerUps Enum" :default "NewEnumerator0"))
  ;[1 1 1] Power Up Activited TODO:Refix the event to make it more efficent
  (switch `/Game/Enums/E_PowerUps` `Power-Up`
    (:`NewEnumerator0`
      (set `self.bInstaKillActive` true)
      (bind _outactors (`GameplayStatics.GetAllActorsOfClass` "/Game/FirstPersonBP/Blueprints/FirstPersonCharacter.FirstPersonCharacter_C"))
      (for _array_element _outactors
        (bind _returnvalue (`|CreateWidget` "/Game/FirstPersonBP/Blueprints/WBP_PowerUp.WBP_PowerUp_C"))
        (set `/Game/FirstPersonBP/Blueprints/WBP_PowerUp.Power-Up` "NewEnumerator0" _returnvalue)
        (`HorizontalBox.AddChildToHorizontalBox` (`/Game/FirstPersonBP/Blueprints/WBP_PlayerHUD.PowerUpImageBox` (`/Game/FirstPersonBP/Blueprints/FirstPersonCharacter.Player HUD Ref` _array_element)) _returnvalue)
        (`KismetSystemLibrary.Delay` 30.0)
        (set `self.bInstaKillActive` false)))
    (:`NewEnumerator1`
      (set `self.bDoublePointsActive` true)
      (bind _outactors_2 (`GameplayStatics.GetAllActorsOfClass` "/Game/FirstPersonBP/Blueprints/FirstPersonCharacter.FirstPersonCharacter_C"))
      (for _array_element_2 _outactors_2
        (bind _returnvalue_2 (`|CreateWidget` "/Game/FirstPersonBP/Blueprints/WBP_PowerUp.WBP_PowerUp_C"))
        (set `/Game/FirstPersonBP/Blueprints/WBP_PowerUp.Power-Up` "NewEnumerator1" _returnvalue_2)
        (`HorizontalBox.AddChildToHorizontalBox` (`/Game/FirstPersonBP/Blueprints/WBP_PlayerHUD.PowerUpImageBox` (`/Game/FirstPersonBP/Blueprints/FirstPersonCharacter.Player HUD Ref` _array_element_2)) _returnvalue_2)
        (`KismetSystemLibrary.Delay` 30.0)
        (set `self.bDoublePointsActive` false)))))

(event `PowerUpActivated`
  (params (PowerUp :type "/Game/Enums/E_PowerUps Enum" :default "NewEnumerator0")))

(fn `Calculate Cat Number`
  (set `self.Cats Left` (- (* (`self.Wave #`) 5) (* (`self.Wave #`) 2))))

(fn `UserConstructionScript`)