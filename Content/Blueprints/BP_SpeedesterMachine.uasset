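; BP_SpeedesterMachine is a purchasable perk machine that sells the Speedester perk to the player for points.
; Its collision box shows a HUD prompt to a FirstPersonCharacter lacking the perk and hides it when they leave.
; The Interact event checks that the player lacks the perk and has enough points, then deducts the cost, activates Speedester and hides the prompt.
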(event `/Game/Blueprints/BP_InteractableActors.Interact`
  (params (InteractingPlayer :type "/Game/FirstPersonBP/Blueprints/FirstPersonCharacter Object Reference"))
  ;[1 1 1] Interacting
  (if (and (not (`/Game/FirstPersonBP/Blueprints/FirstPersonCharacter.Has Speedester Perk?` InteractingPlayer)) (>= (`/Game/FirstPersonBP/Blueprints/FirstPersonCharacter.Points` InteractingPlayer) (`self.Perk Cost`)))
    (`/Game/FirstPersonBP/Blueprints/FirstPersonCharacter.Deduct Points` InteractingPlayer (`self.Perk Cost`))
    (`/Game/FirstPersonBP/Blueprints/FirstPersonCharacter.Activate Speedester` InteractingPlayer)
    (`/Game/FirstPersonBP/Blueprints/WBP_PlayerHUD.Hide Promt Message` (`/Game/FirstPersonBP/Blueprints/FirstPersonCharacter.Player HUD Ref` InteractingPlayer))))

(event `self.Collision Box.OnComponentBeginOverlap`
  (params (OverlappedComponent :type "PrimitiveComponent Object Reference") (OtherActor :type "Actor Object Reference") (OtherComp :type "PrimitiveComponent Object Reference") (OtherBodyIndex :type Integer) (bFromSweep :type Boolean) (SweepResult :type "HitResult Structure (by ref)"))
  (bind _asfirst_person_character (cast `/Game/FirstPersonBP/Blueprints/FirstPersonCharacter` OtherActor))
  (if (not (`/Game/FirstPersonBP/Blueprints/FirstPersonCharacter.Has Speedester Perk?` _asfirst_person_character))
    (`/Game/FirstPersonBP/Blueprints/WBP_PlayerHUD.Show Promt Message` (`/Game/FirstPersonBP/Blueprints/FirstPersonCharacter.Player HUD Ref` _asfirst_person_character) (`self.Promt Message`))))

(event `self.Collision Box.OnComponentEndOverlap`
  (params (OverlappedComponent :type "PrimitiveComponent Object Reference") (OtherActor :type "Actor Object Reference") (OtherComp :type "PrimitiveComponent Object Reference") (OtherBodyIndex :type Integer))
  (bind _asfirst_person_character (cast `/Game/FirstPersonBP/Blueprints/FirstPersonCharacter` OtherActor))
  (`/Game/FirstPersonBP/Blueprints/WBP_PlayerHUD.Hide Promt Message` (`/Game/FirstPersonBP/Blueprints/FirstPersonCharacter.Player HUD Ref` _asfirst_person_character)))

(fn `UserConstructionScript`
  (`parent.UserConstructionScript`))