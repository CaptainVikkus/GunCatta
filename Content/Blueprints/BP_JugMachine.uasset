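; BP_JugMachine is a perk vending machine that sells the Jug perk to players.
; On its Interact event, it checks that the interacting player lacks the perk and has enough points to cover PerkCost.
; It then deducts the points and calls ActivateJug on that player, leaving the perk's effect to the player.
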(event `/Game/Blueprints/BP_InteractableActors.Interact`
  (params (InteractingPlayer :type "/Game/FirstPersonBP/Blueprints/FirstPersonCharacter Object Reference"))
  ;[1 1 1] Interacting
  (if (and (not (`/Game/FirstPersonBP/Blueprints/FirstPersonCharacter.Has Jug Perk?` InteractingPlayer)) (>= (`/Game/FirstPersonBP/Blueprints/FirstPersonCharacter.Points` InteractingPlayer) (`self.Perk Cost`)))
    (`/Game/FirstPersonBP/Blueprints/FirstPersonCharacter.Deduct Points` InteractingPlayer (`self.Perk Cost`))
    (`/Game/FirstPersonBP/Blueprints/FirstPersonCharacter.Activate Jug` InteractingPlayer)))

(fn `UserConstructionScript`
  (`parent.UserConstructionScript`))