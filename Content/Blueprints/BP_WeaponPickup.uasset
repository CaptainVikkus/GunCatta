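; Purchasable weapon pickup that lets an interacting player spend points on a weapon, or on an ammo refill if they already own it.
; A new weapon fills slot 1, then slot 2 with the Third Arm perk, otherwise replaces the current weapon.
; A box overlap shows and hides the HUD buy prompt, using weapon and ammo texts prebuilt in the construction script.
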(event `self.Interact`
  (params (InteractingPlayer :type "/Game/FirstPersonBP/Blueprints/FirstPersonCharacter Object Reference"))
  (bind _weapon_cost (`self.Weapon Cost`))
  (bind _weaponslots (`/Game/FirstPersonBP/Blueprints/FirstPersonCharacter.WeaponSlots` InteractingPlayer))
  (bind _ammo_refill_cost (`self.Ammo Refill Cost`))
  (bind _weapon_ref (`/Game/FirstPersonBP/Blueprints/FirstPersonCharacter.Has Weapon?` InteractingPlayer (`self.Weapon 4 Sale`)))
  ;[1 1 1] First check if the player already has the weapon(buying ammo) or not (buying weapon)
  (if (== _weapon_ref null)
    ;[1 1 1] Check if the player can afford the weapon
    (if (>= (`/Game/FirstPersonBP/Blueprints/FirstPersonCharacter.Points` InteractingPlayer) _weapon_cost)
      (`/Game/FirstPersonBP/Blueprints/FirstPersonCharacter.Deduct Points` InteractingPlayer _weapon_cost)
      ;[1 1 1] Check if there is an open slot for the weapon
      (if (== (`|GetArrayItem` _weaponslots 1) null)
        (`/Game/FirstPersonBP/Blueprints/FirstPersonCharacter.BuildWeapons` InteractingPlayer (`self.Weapon 4 Sale`) 1)
        (elif (and (`/Game/FirstPersonBP/Blueprints/FirstPersonCharacter.Has Third Arm Perk?` InteractingPlayer) (== (`|GetArrayItem` _weaponslots 2) null))
          (`/Game/FirstPersonBP/Blueprints/FirstPersonCharacter.BuildWeapons` InteractingPlayer (`self.Weapon 4 Sale`) 2)
          (else
            ;[1 1 1] If there's no open slot then replace the current weapon with this weapon
            (`/Game/FirstPersonBP/Blueprints/FirstPersonCharacter.BuildWeapons` InteractingPlayer (`self.Weapon 4 Sale`) -1))))
      (`/Game/FirstPersonBP/Blueprints/WBP_PlayerHUD.Show Promt Message` (`/Game/FirstPersonBP/Blueprints/FirstPersonCharacter.Player HUD Ref` InteractingPlayer) (`self.Buy Ammo Promt`)))
    (else
      ;[1 1 1] Check if the player can afford the ammo
      (if (>= (`/Game/FirstPersonBP/Blueprints/FirstPersonCharacter.Points` InteractingPlayer) _ammo_refill_cost)
        (`/Game/FirstPersonBP/Blueprints/FirstPersonCharacter.Deduct Points` InteractingPlayer _ammo_refill_cost)
        ;[1 1 1] Simply refill the weapon's ammo
        (`/Game/FirstPersonBP/Blueprints/BP_Weapon.Fully Refill Weapon` _weapon_ref)))))

(event `self.Box.OnComponentBeginOverlap`
  (params (OverlappedComponent :type "PrimitiveComponent Object Reference") (OtherActor :type "Actor Object Reference") (OtherComp :type "PrimitiveComponent Object Reference") (OtherBodyIndex :type Integer) (bFromSweep :type Boolean) (SweepResult :type "HitResult Structure (by ref)"))
  (bind _asfirst_person_character (cast `/Game/FirstPersonBP/Blueprints/FirstPersonCharacter` OtherActor))
  (if (== (`/Game/FirstPersonBP/Blueprints/FirstPersonCharacter.Has Weapon?` _asfirst_person_character (`self.Weapon 4 Sale`)) null)
    (bind _player_hud_ref (`/Game/FirstPersonBP/Blueprints/FirstPersonCharacter.Player HUD Ref` _asfirst_person_character))
    (`/Game/FirstPersonBP/Blueprints/WBP_PlayerHUD.Show Promt Message` _player_hud_ref (`self.Buy Weapon Promt`))
    (else
      (`/Game/FirstPersonBP/Blueprints/WBP_PlayerHUD.Show Promt Message` _player_hud_ref (`self.Buy Ammo Promt`)))))

(event `self.Box.OnComponentEndOverlap`
  (params (OverlappedComponent :type "PrimitiveComponent Object Reference") (OtherActor :type "Actor Object Reference") (OtherComp :type "PrimitiveComponent Object Reference") (OtherBodyIndex :type Integer))
  (bind _asfirst_person_character (cast `/Game/FirstPersonBP/Blueprints/FirstPersonCharacter` OtherActor))
  (`/Game/FirstPersonBP/Blueprints/WBP_PlayerHUD.Hide Promt Message` (`/Game/FirstPersonBP/Blueprints/FirstPersonCharacter.Player HUD Ref` _asfirst_person_character)))

(fn `UserConstructionScript`
  (set `self.Buy Ammo Promt` (`KismetTextLibrary.Conv_StringToText` (`KismetStringLibrary.Concat_StrStr` "Buy Ammo for  " (`KismetStringLibrary.Conv_IntToString` (`self.Ammo Refill Cost`)) " Points")))
  (set `self.Buy Weapon Promt` (`KismetTextLibrary.Conv_StringToText` (`KismetStringLibrary.Concat_StrStr` "Buy   " (`KismetSystemLibrary.GetClassDisplayName` (`self.Weapon 4 Sale`)) " for " (`KismetStringLibrary.Conv_IntToString` (`self.Weapon Cost`)) " Points"))))